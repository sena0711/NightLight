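; AI character that pairs with another BP_NB_AICharacter for timed NPC conversations.
; SetAIReadyToTalk switches the AI controller to Idle and starts a looping timer that checks distance to TalkingTarget.
; Once in range it flags itself as waiting, and starts talking when the target is also waiting.
; While talking, Tick eases yaw toward the target by a per-frame fraction, until a delay ends the talk and restores Neutral.
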(event `self.ReceiveBeginPlay`)

(event `self.ReceiveTick`
  (params (DeltaSeconds :type "Float (single-precision)"))
  (if (`self.IsTalking`)
    (`self.RotateActor`)))

(event `ToStopTalking`
  (if (`self.IsTalking`)
    (`KismetSystemLibrary.Delay` (`self.CurrentTalkingDuration`))
    (set `self.WaitingForTargetToTalk` false)
    (`self.SetAIReadyToTalk` false)))

(fn `CheckDistanceToTalkingTarget`
  (bind _talkingtarget (`self.TalkingTarget`))
  (if (`self.IsReadyToTalk`)
    (if (<= (`self.GetDistanceTo` self _talkingtarget) 400.0)
      (set `self.WaitingForTargetToTalk` true)
      (bind _asbp_nb_aicharacter (cast `/Game/Blueprints/NPC/BP_NB_AICharacter` _talkingtarget))
      (if (`/Game/Blueprints/NPC/BP_NB_AICharacter.WaitingForTargetToTalk` _asbp_nb_aicharacter)
        (set `self.IsTalking` true)
        (`self.ToStopTalking`)
        (`KismetSystemLibrary.K2_ClearAndInvalidateTimerHandle` (`self.TimeHandlerCheckTalkingTarget`))))))

(fn `RotateActor`
  (bind (_returnvalue_roll _returnvalue_pitch _returnvalue_yaw) (`KismetMathLibrary.BreakRotator` (`self.K2_GetActorRotation`)))
  (bind (_returnvalue_roll_2 _returnvalue_pitch_2 _returnvalue_yaw_2) (`KismetMathLibrary.BreakRotator` (`self.K2_GetActorRotation`)))
  (bind (_returnvalue_roll_3 _returnvalue_pitch_3 _returnvalue_yaw_3) (`KismetMathLibrary.BreakRotator` (`KismetMathLibrary.FindLookAtRotation` (`self.K2_GetActorLocation`) (`self.K2_GetActorLocation` (`self.TalkingTarget`)))))
  (if (not (`KismetMathLibrary.NearlyEqual_FloatFloat` _returnvalue_yaw _returnvalue_yaw_3 2.0))
    (`self.K2_AddActorWorldRotation` (`KismetMathLibrary.MakeRotator` 0.0 0.0 (/ (- _returnvalue_yaw_3 _returnvalue_yaw_2) 50.0)))))

(fn `SetAIReadyToTalk`
  (params (bSetReadyToTalk :type Boolean) (TalkingDuration :type "Float (double-precision)"))
  (set `self.CurrentTalkingDuration` TalkingDuration)
  (if bSetReadyToTalk
    ;[1 1 1] WaitAtLocationToTalk
    (bind _asbp_nb_aicontroller (cast `/Game/Blueprints/NPC/BP_NB_AIController` (`self.GetController`)))
    (`NB_AIController.SetAIBehaviorStateAndKey` _asbp_nb_aicontroller "Idle")
    (set `self.IsReadyToTalk` true)
    (bind _returnvalue (`KismetSystemLibrary.K2_SetTimer` null "CheckDistanceToTalkingTarget" 0.5 true))
    (set `self.TimeHandlerCheckTalkingTarget` _returnvalue)
    (else
      ;[1 1 1] WaitAtLocationToTalk
      (set `self.IsTalking` false)
      (bind _asbp_nb_aicontroller_2 (cast `/Game/Blueprints/NPC/BP_NB_AIController` (`self.GetController`)))
      (`NB_AIController.SetAIBehaviorStateAndKey` _asbp_nb_aicontroller_2 "Neutral")
      (set `self.IsReadyToTalk` false)
      (`KismetSystemLibrary.K2_ClearAndInvalidateTimerHandle` (`self.TimeHandlerCheckTalkingTarget`)))))

(fn `UserConstructionScript`)