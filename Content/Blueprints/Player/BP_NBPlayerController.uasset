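; BP_NBPlayerController is a player controller Blueprint that assigns UI images to the bullet items it references.
; InitializeBulletItemsUIimages loops over BulletItems, switches on each item's bullet type, and picks the Standard or Light UI image.
; Each struct is written back at its index with possessed value and type preserved.
; Tick and the construction script are empty.
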(event `self.ReceiveTick`
  (params (DeltaSeconds :type "Float (single-precision)")))

(event `self.InitializeBulletItemsUIimages`
  (for (_array_element _array_index) (`self.BulletItems`)
    (switch `EBulletType` (`.BulletType` (break `BulletItem` _array_element))
      (:`EStandard`
        (bind (_currentpossesed _bullettype) (break `BulletItem` _array_element))
        (`KismetArrayLibrary.Array_Set` (`self.BulletItems`) _array_index (make `BulletItem` _currentpossesed _bullettype (`self.StandardBulletUI`))))
      (:`ELight`
        (bind (_currentpossesed_2 _bullettype_2) (break `BulletItem` _array_element))
        (`KismetArrayLibrary.Array_Set` (`self.BulletItems`) _array_index (make `BulletItem` _currentpossesed_2 _bullettype_2 (`self.LightBulletUI`)))))))

(fn `UserConstructionScript`)