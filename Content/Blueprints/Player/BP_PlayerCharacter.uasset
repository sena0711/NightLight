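; Player character Blueprint that drives head-look, body turning and the carry point for physics-held objects.
; Tick moves the PhysicsHandle target to HoldingPoint, derives HeadRotation from control versus actor rotation, and flags left or right mouse input to stop past the yaw limit.
; When RotateActor is set, the body interpolates toward the view yaw and clears those flags.
; Key 0 prints the controller's current grabbable and pickupable; grab, release and spring-arm attach nodes are unconnected.
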(event `self.ReceiveBeginPlay`)

(event `Key|Zero`
  (params (Key :type "Key Structure"))
  (:`Pressed`
    (bind _asbp_nbplayer_controller (cast `/Game/Blueprints/Player/BP_NBPlayerController` (`self.GetController`)))
    (`KismetSystemLibrary.PrintString` (`KismetSystemLibrary.GetDisplayName` (`NBPlayerController.CurrentGrabable` _asbp_nbplayer_controller)) true true (struct :`R` 1.0 :`G` 0.276001 :`B` 0.216254 :`A` 1.0))
    (`KismetSystemLibrary.PrintString` (`KismetSystemLibrary.GetDisplayName` (`NBPlayerController.CurrentPickupable` _asbp_nbplayer_controller)))))

(event `self.ReceiveTick`
  (params (DeltaSeconds :type "Float (single-precision)"))
  (bind (_returnvalue_roll _returnvalue_pitch _returnvalue_yaw) (`KismetMathLibrary.BreakRotator` (`self.GetControlRotation`)))
  (bind (_returnvalue_roll_2 _returnvalue_pitch_2 _returnvalue_yaw_2) (`KismetMathLibrary.BreakRotator` (`self.K2_GetActorRotation`)))
  (bind (_returnvalue_roll_3 _returnvalue_pitch_3 _returnvalue_yaw_3) (`KismetMathLibrary.BreakRotator` (`self.K2_GetActorRotation`)))
  (bind _returnvalue (`KismetMathLibrary.ClampAngle` (- _returnvalue_yaw _returnvalue_yaw_2) -170.0 -180.0))
  ;[1 1 1] Set Physics Handle Location
  (`PhysicsHandleComponent.SetTargetLocation` (`self.PhysicsHandle`) (`SceneComponent.K2_GetComponentLocation` (`self.HoldingPoint`)))
  ;[1 1 1] HeadRotation
  ;;[1 0.9933 0.2622] Set Head Rotation
  (set `self.HeadRotation` (`KismetMathLibrary.MakeRotator` (- 0.0 _returnvalue_pitch) 0.0 _returnvalue))
  ;;[1 0.9933 0.2622] PutLimitation on  Head Rotation
  (if (> _returnvalue (`self.MaxAllowedHeadRotationAngle`))
    (set `self.bStopLeftMouseInput` false)
    (set `self.bStopRightMouseInput` true)
    (elif (< _returnvalue (* (`self.MaxAllowedHeadRotationAngle`) -1.0))
      (set `self.bStopRightMouseInput` false)
      (set `self.bStopLeftMouseInput` true)
      (else
        (set `self.bStopRightMouseInput` false)
        (set `self.bStopLeftMouseInput` false))))
  ;;[1 0.9933 0.2622] Actor Rotation
  (if (`self.bRotateActor`)
    (set `self.DesiredActorYaw` (+ _returnvalue_yaw_3 (`self.LocalActorYawOffset`)))
    (set `self.LocalActorYawOffset` _returnvalue)
    (`self.K2_SetActorRotation` (`KismetMathLibrary.RInterpTo` (`self.K2_GetActorRotation`) (`KismetMathLibrary.MakeRotator` 0.0 0.0 (`self.DesiredActorYaw`)) (`GameplayStatics.GetWorldDeltaSeconds`) 5.0))
    (set `self.bStopLeftMouseInput` false)
    (set `self.bStopRightMouseInput` false)))

(fn `UserConstructionScript`)