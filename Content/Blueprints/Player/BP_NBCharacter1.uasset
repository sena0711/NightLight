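; First-person player character that carries grabbed objects, limits head look and mounts torch and weapon on arm sockets.
; Tick moves the physics handle to the holding point for holdables or the camera trace end otherwise, also driving grabbed drawers.
; Yaw and pitch limits set mouse-input stop flags.
; Turn-in-spot and arm sway trigger ActorRotation, which interpolates the body toward the control yaw offset.
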(event `self.ReceiveTick`
  (params (DeltaSeconds :type "Float (single-precision)"))
  (bind (_returnvalue_roll _returnvalue_pitch _returnvalue_yaw) (`KismetMathLibrary.BreakRotator` (`self.K2_GetActorRotation`)))
  (bind (_returnvalue_roll_2 _returnvalue_pitch_2 _returnvalue_yaw_2) (`KismetMathLibrary.BreakRotator` (`self.GetControlRotation`)))
  (bind (_hitresultfromcameracenter_bblockinghit _hitresultfromcameracenter_binitialoverlap _hitresultfromcameracenter_time _hitresultfromcameracenter_distance _hitresultfromcameracenter_location _hitresultfromcameracenter_impactpoint _hitresultfromcameracenter_normal _hitresultfromcameracenter_impactnormal _hitresultfromcameracenter_physmat _hitresultfromcameracenter_hitactor _hitresultfromcameracenter_hitcomponent _hitresultfromcameracenter_hitbonename _hitresultfromcameracenter_hititem _hitresultfromcameracenter_faceindex _hitresultfromcameracenter_tracestart _hitresultfromcameracenter_traceend) (`GameplayStatics.BreakHitResult` (`self.HitResultFromCameraCenter`)))
  (bind _returnvalue (- _returnvalue_pitch_2 _returnvalue_pitch))
  (bind _returnvalue_2 (* (`self.MaxAllowedHeadRotationAngle`) -1.0))
  (bind _returnvalue_3 (`KismetMathLibrary.ClampAngle` (- _returnvalue_yaw_2 _returnvalue_yaw) -170.0 -180.0))
  (`|ExecutionSequence`
    (:`then_0`
      ;[0.7292 1 0.6607] Picking up Holding obj
      (bind _asbp_nbplayer_controller (cast `/Game/Blueprints/Player/BP_NBPlayerController` (`GameplayStatics.GetPlayerController` 0)))
      (bind _currentgrabable (`NBPlayerController.CurrentGrabable` _asbp_nbplayer_controller))
      (`/Engine/EditorBlueprintResources/StandardMacros.IsValid` _currentgrabable
        (:`Is Valid`
          (if (`BaseGrabable.bHoldable` _currentgrabable)
            ;;[0.04025 0.5884 1] Set Physics Handle Location to Holding Point
            (`PhysicsHandleComponent.SetTargetLocation` (`self.PhysicsHandle`) (`SceneComponent.K2_GetComponentLocation` (`self.HoldingPoint`)))
            (else
              ;;[0.04025 0.5884 1] Set Physics Handle Location : follows mouse
              (`PhysicsHandleComponent.SetTargetLocation` (`self.PhysicsHandle`) _hitresultfromcameracenter_traceend)
              ;;[0.04025 0.5884 1] if current grabable is drawer
              (bind _asbp_nbplayer_controller_2 (cast `/Game/Blueprints/Player/BP_NBPlayerController` (`GameplayStatics.GetPlayerController` 0)))
              (bind _asgrab_drawer (cast `/Game/Blueprints/Assets/Grab_Drawer` (`NBPlayerController.CurrentGrabable` _asbp_nbplayer_controller_2)))
              (if (`self.HoldingObject`)
                (set `self.CameraSensitivity` (`self.HoldingCameraSensitivity`))
                (`/Game/Blueprints/Assets/Grab_Drawer.MoveDrawer` _asgrab_drawer (`self.LookingDirection`))))))))
    (:`then_1`
      ;[1 1 1] CameraRotation
      ;;[1 0.9933 0.2622] PutLimitation on  Head Rotation
      (set `self.LocalActorYawOffset` _returnvalue_3)
      (if (> _returnvalue_3 (`self.MaxAllowedHeadRotationAngle`))
        (set `self.LocalActorYawOffset` (`self.MaxAllowedHeadRotationAngle`))
        (set `self.bStopLeftMouseInput` false)
        (set `self.bStopRightMouseInput` true)
        (if (`self.TurningInSpotAllowed`) :!label _label
          (set `self.bRotateActor` true)
          (`self.ActorRotation` (`self.bRotateActor`))
          (else
            (`self.ActorRotation` (`self.bRotateActor`))))
        (elif (< _returnvalue_3 _returnvalue_2)
          (set `self.LocalActorYawOffset` _returnvalue_2)
          (set `self.bStopRightMouseInput` false)
          (set `self.bStopLeftMouseInput` true)
          (goto _label)
          (else
            (set `self.bStopRightMouseInput` false)
            (set `self.bStopLeftMouseInput` false)
            (`self.ActorRotation` (`self.bRotateActor`))))))
    (:`then_2`
      ;;[1 0.9933 0.2622] Enable Sway (Arm movement
      (if (`self.EnableSway`)
        (if (not (`KismetMathLibrary.NearlyEqual_FloatFloat` _returnvalue_3 0.0 0.001))
          (set `self.bRotateActor` true)
          (`self.ActorRotation` (`self.bRotateActor`)))))
    (:`then_3`
      ;;[1 0.9933 0.2622] Limitate Pitch Rotation
      (if (>= _returnvalue 250.0)
        (if (<= _returnvalue 320.0)
          (set `self.bStopDownMouseInput` true)
          (else
            (set `self.bStopDownMouseInput` false :!label _label_2)))
        (else
          (goto _label_2))))))

(event `self.AttachTorchToGun`
  (bind _currenttorch (`self.CurrentTorch`))
  ;[1 0.5895 0.1834] Attach Torch to hand
  (`|ExecutionSequence`
    (:`then_0`
      (`/Engine/EditorBlueprintResources/StandardMacros.IsValid` _currenttorch
        (:`Is Valid`
          (`self.K2_AttachToComponent` _currenttorch (`self.ArmMesh`) "Torch_Socket" "SnapToTarget" "SnapToTarget" "SnapToTarget" true))))
    (:`then_1`
      (`/Engine/EditorBlueprintResources/StandardMacros.IsValid` (`self.CurrentWeapon`)
        (:`Is Valid`
          (`self.K2_AttachToComponent` (`self.CurrentWeapon`) (`self.ArmMesh`) "Weapon_Socket" "SnapToTarget" "SnapToTarget" "SnapToTarget" true))))))

(fn `ActorRotation`
  (params (SetNewRotation :type Boolean))
  (bind (_returnvalue_roll _returnvalue_pitch _returnvalue_yaw) (`KismetMathLibrary.BreakRotator` (`self.K2_GetActorRotation`)))
  ;[1 0.9933 0.2622] Actor Rotation
  (if SetNewRotation
    (set `self.DesiredActorYaw` (+ _returnvalue_yaw (`self.LocalActorYawOffset`)))
    (`self.K2_SetActorRotation` (`KismetMathLibrary.RInterpTo` (`self.K2_GetActorRotation`) (`KismetMathLibrary.MakeRotator` 0.0 0.0 (`self.DesiredActorYaw`)) (`GameplayStatics.GetWorldDeltaSeconds`) 5.0))
    (set `self.bStopLeftMouseInput` false)
    (set `self.bStopRightMouseInput` false)))

(fn `UserConstructionScript`)