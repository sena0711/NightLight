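; Actor component that plays footstep sounds for the owning BP_PlayerCharacter based on distance moved.
; Each tick, once the actor is farther than Stride from the last footstep point while moving on ground, it line-traces downward on Visibility.
; If the hit physical material is Floor, it plays the footstep cue at the impact location and stores that point for the next distance check.
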(event `self.ReceiveTick`
  (params (DeltaSeconds :type "Float (single-precision)"))
  (bind _player_character_ref (`self.Player Character Ref`))
  (bind _returnvalue (`Actor.K2_GetActorLocation` _player_character_ref))
  (bind _asbp_player_character (cast `/Game/Blueprints/Player/BP_PlayerCharacter` (`self.GetOwner`)))
  (bind _output_get (set `self.Player Character Ref` _asbp_player_character))
  (if (and (> (`KismetMathLibrary.VSize` (- (`Actor.K2_GetActorLocation` (`self.Player Character Ref`)) (`self.Last Footstep Location`))) (`self.Stride`)) (`NavMovementComponent.IsMovingOnGround` (`Pawn.GetMovementComponent` _output_get)))
    (bind (_outhit _returnvalue_2) (`KismetSystemLibrary.LineTraceSingle` _returnvalue (- _returnvalue (`KismetMathLibrary.MakeVector` 0.0 0.0 (* (`CapsuleComponent.CapsuleHalfHeight` (`Character.CapsuleComponent` _player_character_ref)) 2.0))) "TraceTypeQuery1"))
    (bind (_bblockinghit _binitialoverlap _time _distance _location _impactpoint _normal _impactnormal _physmat) (`GameplayStatics.BreakHitResult` _outhit))
    (if (and _returnvalue_2 (== _physmat "/Game/Material/Phys_Materials/Floor.Floor"))
      (`GameplayStatics.PlaySoundAtLocation` "/Game/Sound/Footsteps/FootstepSoundCue.FootstepSoundCue" _location)
      (set `self.Last Footstep Location` _location))))