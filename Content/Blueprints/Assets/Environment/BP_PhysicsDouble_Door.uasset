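; Physics-driven double door that snaps each leaf back to its starting rotation when it swings near it.
; BeginPlay enables physics on SecondaryMesh and records both door meshes' starting relative rotations.
; Tick snaps each mesh exactly to that rotation once it is nearly aligned and its Z angular velocity is under a threshold.
; Focus events toggle the in-view state of both doors and always clear it on PickupMesh.
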(event `self.ReceiveBeginPlay`
  (`parent.ReceiveBeginPlay`)
  (`PrimitiveComponent.SetSimulatePhysics` (`self.SecondaryMesh`) true)
  (set `self.SecondaryMeshStartingRotation` (`SceneComponent.RelativeRotation` (`self.SecondaryMesh`)))
  (set `self.StaticMeshStartingRotation` (`SceneComponent.RelativeRotation` (`self.StaticMesh`))))

(event `self.ReceiveTick`
  (params (DeltaSeconds :type "Float (single-precision)"))
  (`parent.ReceiveTick` DeltaSeconds)
  (`|ExecutionSequence`
    (:`then_0`
      (`self.SelectedMeshBackToSetRotation` (`self.SecondaryMesh`) (`self.SecondaryMeshStartingRotation`)))
    (:`then_1`
      (`self.SelectedMeshBackToSetRotation` (`self.StaticMesh`) (`self.StaticMeshStartingRotation`)))))

(event `self.InFocus`
  (`self.NotInView` (`self.PickupMesh`))
  (`self.InView` (`self.SecondaryMesh`))
  (`self.InView` (`self.StaticMesh`)))

(event `self.NotInFocus`
  (`self.NotInView` (`self.PickupMesh`))
  (`self.NotInView` (`self.SecondaryMesh`))
  (`self.NotInView` (`self.StaticMesh`)))

(fn `SelectedMeshBackToSetRotation`
  (params (Mesh :type "SceneComponent Object Reference") (RoationTo :type "Rotator Structure"))
  ;[1 1 1] Set selected Mesh back to set rotation
  (bind _asprimitive_component (cast `PrimitiveComponent` Mesh))
  (bind _returnvalue (`PrimitiveComponent.GetPhysicsAngularVelocityInDegrees` _asprimitive_component "None"))
  (if (<= (.z _returnvalue) 40.0)
    (if (== (`SceneComponent.RelativeRotation` Mesh) RoationTo :`ErrorTolerance` 1.0)
      (`SceneComponent.K2_SetRelativeRotation` Mesh RoationTo false false))))

(fn `UserConstructionScript`
  (`parent.UserConstructionScript`))