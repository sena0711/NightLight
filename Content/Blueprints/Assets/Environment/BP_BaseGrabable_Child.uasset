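; Grabbable environment prop that extends a parent Blueprint, likely BP_BaseGrabable, with a second physics-driven mesh.
; On BeginPlay, after the parent logic, it re-applies SecondaryMesh's current world location and turns on its physics simulation.
; Focus events pass both PickupMesh and SecondaryMesh to InView or NotInView, so the two highlight together.
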(event `self.ReceiveBeginPlay`
  (bind _secondarymesh (`self.SecondaryMesh`))
  (`parent.ReceiveBeginPlay`)
  (`SceneComponent.K2_SetWorldLocation` _secondarymesh (`SceneComponent.K2_GetComponentLocation` _secondarymesh) false false)
  (`PrimitiveComponent.SetSimulatePhysics` _secondarymesh true))

(event `self.InFocus`
  ;[1 1 1] HighLight
  (`self.InView` (`self.PickupMesh`))
  (`self.InView` (`self.SecondaryMesh`)))

(event `self.NotInFocus`
  ;[1 1 1] HighLight
  (`self.NotInView` (`self.PickupMesh`))
  (`self.NotInView` (`self.SecondaryMesh`)))

(fn `UserConstructionScript`
  (`parent.UserConstructionScript`))