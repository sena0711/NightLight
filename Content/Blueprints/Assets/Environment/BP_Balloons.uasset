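; Balloons environment actor that plays an impact sound when its Balloons component is hit.
; The hit event limits playback to once per half second and skips hits while the Audio component is still playing.
; Volume is meant to follow impact intensity but divides the impact normal's length by SoundMultiplier, so it stays effectively constant for a given multiplier.
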(event `self.Balloons.OnComponentHit`
  (params (HitComponent :type "PrimitiveComponent Object Reference") (OtherActor :type "Actor Object Reference") (OtherComp :type "PrimitiveComponent Object Reference") (NormalImpulse :type "Vector Structure") (Hit :type "HitResult Structure (by ref)"))
  (bind _audio (`self.Audio`))
  (if (>= (- (`GameplayStatics.GetTimeSeconds`) (`self.LastPlayedTime`)) 0.5)
    ;[1 1 1] Play sound when hit
    (if (not (`AudioComponent.IsPlaying` _audio))
      (`AudioComponent.SetSound` _audio (`self.SoundHit`))
      (set `AudioComponent.VolumeMultiplier` (/ (`KismetMathLibrary.VSize` Hit_ImpactNormal) (`self.SoundMultiplier`)) (`self.Audio`))
      (`AudioComponent.Play` _audio 0.0)
      (set `self.LastPlayedTime` (`GameplayStatics.GetTimeSeconds`)))))

(fn `UserConstructionScript`)