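; BP_PhysicsDouble is an environment actor with two physics-driven meshes, Left and Right, that can settle back to a resting rotation.
; BeginPlay stores both starting rotations, and each Tick runs SelectedMeshBackToSetRotation on each mesh.
; That function snaps a mesh to the target once Z angular velocity is at most a threshold and rotation is nearly matching.
; Both meshes target Left's starting rotation, leaving Right's stored value unused.
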(event `self.ReceiveBeginPlay`
  (set `self.LeftStartingRotation` (`SceneComponent.RelativeRotation` (`self.Left`)))
  (set `self.RightStartingRotation` (`SceneComponent.RelativeRotation` (`self.Right`))))

(event `self.ReceiveTick`
  (params (DeltaSeconds :type "Float (single-precision)"))
  (`self.SelectedMeshBackToSetRotation` (`self.Left`) (`self.LeftStartingRotation`))
  (`self.SelectedMeshBackToSetRotation` (`self.Right`) (`self.LeftStartingRotation`)))

(fn `SelectedMeshBackToSetRotation`
  (params (Mesh :type "SceneComponent Object Reference") (RotationToGoBack :type "Rotator Structure"))
  ;[1 1 1] Set selected Mesh back to set rotation
  (bind _asprimitive_component (cast `PrimitiveComponent` Mesh))
  (bind _returnvalue (`PrimitiveComponent.GetPhysicsAngularVelocityInDegrees` _asprimitive_component "None"))
  (if (<= (.z _returnvalue) 40.0)
    (if (== (`SceneComponent.RelativeRotation` Mesh) RotationToGoBack :`ErrorTolerance` 1.0)
      (`SceneComponent.K2_SetRelativeRotation` Mesh RotationToGoBack false false))))

(fn `UserConstructionScript`)