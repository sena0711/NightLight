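; Double door actor with two mass-weighted meshes, set heavy so the leaves open and close slowly.
; BeginPlay stores each leaf's starting rotation and overrides its mass with MassKg.
; Every Tick, a shared helper snaps each leaf back to that rotation once it is within a small tolerance.
; Focus events toggle the post-process view state on both leaves, while PickupMesh always stays out of view.
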(event `self.InFocus`
  ;[1 1 1] postprocess
  (`self.NotInView` (`self.PickupMesh`))
  (`self.InView` (`self.SecondaryMesh`))
  (`self.InView` (`self.StaticMesh`)))

(event `self.NotInFocus`
  ;[1 1 1] postprocess
  (`self.NotInView` (`self.PickupMesh`))
  (`self.NotInView` (`self.SecondaryMesh`))
  (`self.NotInView` (`self.StaticMesh`)))

(event `self.ReceiveBeginPlay`
  (bind _masskg (`self.MassKg`))
  (`parent.ReceiveBeginPlay`)
  (`|ExecutionSequence`
    (:`then_0`
      ;[1 1 1] Set Private values
      (set `self.SecondaryMeshStartingRotation` (`SceneComponent.RelativeRotation` (`self.SecondaryMesh`)))
      (set `self.StaticMeshStartingRotation` (`SceneComponent.RelativeRotation` (`self.StaticMesh`))))
    (:`then_1`
      ;[1 1 1] Set door's weight to high so it opens and close slow
      (`PrimitiveComponent.SetMassOverrideInKg` (`self.SecondaryMesh`) "None" _masskg true)
      (`PrimitiveComponent.SetMassOverrideInKg` (`self.StaticMesh`) "None" _masskg true))))

(event `self.ReceiveTick`
  (params (DeltaSeconds :type "Float (single-precision)"))
  (`parent.ReceiveTick` DeltaSeconds)
  (`|ExecutionSequence`
    (:`then_0`
      ;[1 1 1] Go back to begining rotation
      (`self.SelectedMeshBackToSetRotation` (`self.SecondaryMesh`) (`self.SecondaryMeshStartingRotation`)))
    (:`then_1`
      (`self.SelectedMeshBackToSetRotation` (`self.StaticMesh`) (`self.StaticMeshStartingRotation`)))))

(fn `SelectedMeshBackToSetRotation`
  (params (Mesh :type "SceneComponent Object Reference") (RoationTo :type "Rotator Structure"))
  ;[1 1 1] Set selected Mesh back to set rotation
  (cast `PrimitiveComponent` Mesh)
  (if (== (`SceneComponent.RelativeRotation` Mesh) RoationTo :`ErrorTolerance` 3.0)
    (`SceneComponent.K2_SetRelativeRotation` Mesh RoationTo false false)))

(fn `UserConstructionScript`
  (`parent.UserConstructionScript`))