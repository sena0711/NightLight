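; BP_BaseLight_Child is a light actor derived from a base light Blueprint that drives its point light's visibility.
; Every tick it runs the parent tick, calls ProcessLight and applies the boolean result to the PointLight's visibility.
; The WheninLight and WhenNotinLight events only print placeholder debug messages, and the construction script just calls the parent's.
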(event `self.ReceiveTick`
  (params (DeltaSeconds :type "Float (single-precision)"))
  (`parent.ReceiveTick` DeltaSeconds)
  (bind _returnvalue (`self.ProcessLight` true))
  (`SceneComponent.SetVisibility` (`self.PointLight`) _returnvalue false))

(event `self.WhenInLight`
  (`KismetSystemLibrary.PrintString` "Hello"))

(event `self.WhenNotInLight`
  (`KismetSystemLibrary.PrintString` "Bye"))

(fn `UserConstructionScript`
  (`parent.UserConstructionScript`))