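; Grabbable physics drawer door that swings freely once grabbed and latches when it returns to its closed rotation.
; Grabbing while Close is set enables physics on PickupMesh, then arms RestrictDoor after a short delay; otherwise it only sets Close.
; While armed, Tick watches for near-zero relative rotation, then stops physics, snaps shut and resets both flags.
; Focus events toggle the highlight on SecondaryMesh.
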(event `self.ReceiveBeginPlay`
  (`parent.ReceiveBeginPlay`)
  (`PrimitiveComponent.SetSimulatePhysics` (`self.PickupMesh`) false))

(event `self.ReceiveTick`
  (params (DeltaSeconds :type "Float (single-precision)"))
  (bind _pickupmesh (`self.PickupMesh`))
  (`parent.ReceiveTick` DeltaSeconds)
  (if (`self.RestrictDoor`)
    (if (== (`SceneComponent.RelativeRotation` _pickupmesh) (struct) :`ErrorTolerance` 1.0)
      (`PrimitiveComponent.SetSimulatePhysics` _pickupmesh false)
      (`SceneComponent.K2_SetRelativeRotation` :`self` _pickupmesh)
      (set `self.RestrictDoor` false)
      (set `self.Close` true))))

(event `self.WhenGrabbed`
  (if (`self.Close`)
    (set `self.Close` false)
    (`PrimitiveComponent.SetSimulatePhysics` (`self.PickupMesh`) true)
    (`KismetSystemLibrary.Delay` 0.2)
    (set `self.RestrictDoor` true)
    (else
      (set `self.Close` true))))

(event `self.InFocus`
  ;[1 1 1] When the object is in focus we highlight the object
  (`self.InView` (`self.SecondaryMesh`)))

(event `self.NotInFocus`
  ;[1 1 1] When the object is in focus we highlight the object
  (`self.NotInView` (`self.SecondaryMesh`)))

(fn `UserConstructionScript`
  (`parent.UserConstructionScript`))