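; Torch pickup item, built on a parent class, whose mesh starts simulating physics when play begins.
; On interaction it calls PlaySequence, which, despite its name, only destroys the actor referenced by NewVar0 if that reference is valid.
; Overlap and Tick events are disabled, and the construction script only calls the parent.
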(event `self.ReceiveBeginPlay`
  (`parent.ReceiveBeginPlay`)
  (`PrimitiveComponent.SetSimulatePhysics` (`self.PickupMesh`) true))

(event `self.WhenInteracted`
  (`self.PlaySequence`))

(event `PlaySequence`
  (bind _newvar_0 (`self.NewVar_0`))
  (`/Engine/EditorBlueprintResources/StandardMacros.IsValid` _newvar_0
    (:`Is Valid`
      (`self.K2_DestroyActor` _newvar_0))))

(fn `UserConstructionScript`
  (`parent.UserConstructionScript`))