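; Pickup item Blueprint that gives each kind of collectible its "F: Pick up" interaction prompt.
; On BeginPlay it runs the parent logic, then switches on ItemType to set InteractText for keys, supplies, equipment, quest items and instruction pages.
; The graph contains no collection logic, its overlap and tick events are disabled, and the construction script only calls the parent.
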(event `self.ReceiveBeginPlay`
  (`parent.ReceiveBeginPlay`)
  (switch `EItemType` (`self.ItemType`)
    (:`Key`
      (set `self.InteractText` "F: Pick up Key"))
    (:`Health`
      (set `self.InteractText` "F: Pick up HealthPack"))
    (:`Battery`
      (set `self.InteractText` "F: Pick up Batteries"))
    (:`Bullets`
      (set `self.InteractText` "F: Pick up Bullets"))
    (:`Torch`
      (set `self.InteractText` "F: Pick up Torch"))
    (:`Weapon`
      (set `self.InteractText` "F: Pick up Weapon"))
    (:`Quest`
      (set `self.InteractText` "F: Pick up Item"))
    (:`Instruction`
      (set `self.InteractText` "F: Pick up Page"))))

(fn `UserConstructionScript`
  (`parent.UserConstructionScript`))