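; Grabbable hinged door, named as a drawer door, that swings open and closed according to a look up or down input.
; BeginPlay stores the mesh's starting rotation as the closed position.
; Each MoveDrawer call rotates PickupMesh one degree, with looking down opening it and looking up closing it.
; OpenAllowed and CloseAllowed flags, updated after each step, limit travel between the closed pose and about 100 degrees of yaw.
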(event `self.ReceiveBeginPlay`
  (`parent.ReceiveBeginPlay`)
  (set `self.BeginRelativeRot` (`SceneComponent.RelativeRotation` (`self.PickupMesh`))))

(event `self.ReceiveTick`
  (params (DeltaSeconds :type "Float (single-precision)"))
  (`parent.ReceiveTick` DeltaSeconds))

(event `self.MoveDrawer`
  (params (NewParam :type "ELookingDirection Enum" :default "LookingUp"))
  (bind _pickupmesh (`self.PickupMesh`))
  (bind (_beginrelativerot_roll _beginrelativerot_pitch _beginrelativerot_yaw) (`KismetMathLibrary.BreakRotator` (`self.BeginRelativeRot`)))
  (bind (_relativerotation_roll _relativerotation_pitch _relativerotation_yaw) (`KismetMathLibrary.BreakRotator` (`SceneComponent.RelativeRotation` _pickupmesh)))
  (switch `ELookingDirection` NewParam
    (:`LookingUp`
      (if (`self.CloseAllowed`)
        (`SceneComponent.K2_AddRelativeRotation` (`self.PickupMesh`) (struct :`Yaw` -1.0) false false)
        (if (== (`SceneComponent.RelativeRotation` (`self.PickupMesh`)) (`self.BeginRelativeRot`) :`ErrorTolerance` 0.5)
          (set `self.CloseAllowed` false)
          (set `self.OpenAllowed` true)
          (else
            (if (<= (- _beginrelativerot_yaw _relativerotation_yaw) -100.0) :!label _label
              (set `self.CloseAllowed` true)
              (set `self.OpenAllowed` false)
              (else
                (set `self.CloseAllowed` true)
                (set `self.OpenAllowed` true)))))))
    (:`LookingDown`
      (if (`self.OpenAllowed`)
        (`SceneComponent.K2_AddRelativeRotation` _pickupmesh (struct :`Yaw` 1.0) false false)
        (goto _label)))))

(fn `UserConstructionScript`
  (`parent.UserConstructionScript`))