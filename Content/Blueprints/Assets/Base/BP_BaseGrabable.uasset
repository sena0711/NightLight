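; Base grabbable actor that highlights its pickup mesh when in focus and plays impact sounds.
; InFocus and NotinFocus toggle the mesh's custom depth rendering through InView and NotInView.
; On hit, it updates the player controller's CurrentGrabable highlight and, unless muted or already playing, plays SoundHit with volume scaled by impulse.
; A separate time-throttled hit-sound function exists but is not called here.
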(event `self.ReceiveTick`
  (params (DeltaSeconds :type "Float (single-precision)")))

(event `self.InFocus`
  ;[1 1 1] HighLight
  (`self.InView` (`self.PickupMesh`)))

(event `self.NotInFocus`
  ;[1 1 1] HighLight
  (`self.NotInView` (`self.PickupMesh`)))

(event `self.ReceiveHit`
  (params (MyComp :type "PrimitiveComponent Object Reference") (Other :type "Actor Object Reference") (OtherComp :type "PrimitiveComponent Object Reference") (bSelfMoved :type Boolean) (HitLocation :type "Vector Structure") (HitNormal :type "Vector Structure") (NormalImpulse :type "Vector Structure") (Hit :type "HitResult Structure (by ref)"))
  (bind _audio (`self.Audio`))
  ;[1 1 1] Check using hit doing inview out view
  (`|ExecutionSequence`
    (:`then_0`
      (bind _asbp_nbplayer_controller (cast `/Game/Blueprints/Player/BP_NBPlayerController` (`GameplayStatics.GetPlayerController` 0)))
      (bind _currentgrabable (`NBPlayerController.CurrentGrabable` _asbp_nbplayer_controller))
      (`/Engine/EditorBlueprintResources/StandardMacros.IsValid` _currentgrabable
        (:`Is Valid`
          (bind _pickupmesh (`BaseMovable.PickupMesh` _currentgrabable))
          (`/Engine/EditorBlueprintResources/StandardMacros.IsValid` _pickupmesh
            (:`Is Valid`
              (if (== _currentgrabable self)
                (`self.InView` _pickupmesh)
                (else
                  (`self.NotInView` _pickupmesh))))))))
    (:`then_1`
      ;[1 1 1] Play sound when hit
      (if (`self.PickupMeshMuted`)
        _
        (elif (not (`AudioComponent.IsPlaying` _audio))
          (`AudioComponent.SetSound` _audio (`self.SoundHit`))
          (set `AudioComponent.VolumeMultiplier` (/ (`KismetMathLibrary.VSize` NormalImpulse) 10000.0) (`self.Audio`))
          (`AudioComponent.Play` _audio 0.0))))))

(fn `InView`
  (params (selfMesh :type "PrimitiveComponent Object Reference"))
  (`/Engine/EditorBlueprintResources/StandardMacros.IsValid` selfMesh
    (:`Is Valid`
      (`PrimitiveComponent.SetRenderCustomDepth` selfMesh true))))

(fn `NotInView`
  (params (selfMesh :type "PrimitiveComponent Object Reference"))
  (`/Engine/EditorBlueprintResources/StandardMacros.IsValid` selfMesh
    (:`Is Valid`
      (`PrimitiveComponent.SetRenderCustomDepth` selfMesh false))))

(fn `PlaySoundWhenComponentIsHit`
  (params (Impact :type "Vector Structure") (HitSound :type "SoundBase Object Reference"))
  (bind _audio (`self.Audio`))
  (if (> (- (`GameplayStatics.GetTimeSeconds`) (`self.LastPlayedTime`)) (`self.Duration`))
    ;[1 1 1] Play sound when hit
    (set `AudioComponent.VolumeMultiplier` (/ (`KismetMathLibrary.VSize` Impact) 30.0) _audio)
    (`AudioComponent.SetSound` _audio HitSound)
    (`AudioComponent.Play` _audio 0.0)
    (set `self.LastPlayedTime` (`GameplayStatics.GetTimeSeconds`))))

(fn `UserConstructionScript`)